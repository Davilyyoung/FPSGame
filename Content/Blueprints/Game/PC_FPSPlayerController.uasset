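; Player controller for a multiplayer deathmatch shooter, bridging the server game mode and each player's HUD.
; It creates the local UI, forwarding ammo, health, crosshair recoil and a sorted scoreboard, and stores the match countdown.
; Spawning is requested from BP_DeathShootGameMode, initially after a delay, and the controller possesses the new pawn.
; Death reports victim and killer, disables input, destroys the pawn and requests respawn; game end opens the main menu.
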(event Custom|SpawnPlayerCharator
  (params (Class :type BP%20Player%20Pawn%20Class%20Reference) (SpawnTransform :type Transform))
  ;[1 1 1] SpawnActor
  ;;[0.6337 0.6143 1] 生成玩家
  (bind _returnvalue (Game|SpawnActorfromClass Class SpawnTransform "Undefined" 0 0)) ; Class生成谁。Spawn Transform生成的位子。从服务器端拿
  (Pawn|Possess _returnvalue) ; 把生成的东西作为，被PlayerController控制的Pawn
  (CallFunction|ClientHidMouse))

(event Custom|StartSpawnCharator
  ;[1 1 1] SpawnActor
  ;;[0.6337 0.6143 1] 玩家加入后会等1秒 GameMode里生成玩家的时候调用此方法 在把玩家创建出来 防止枪械还没加载完毕
  (Utilities|FlowControl|Delay 1.0) ; 延迟1秒
  (bind _asbp_death_shoot_game_mode (Utilities|Casting|CastToBP_DeathShootGameMode (Game|GetGameMode))) ; 拿到我们自己的GameMode
  (Utilities|IsValid _asbp_death_shoot_game_mode ; 判断是否拿到
    (:Is%20Valid
      (Default|RequstSpawn _asbp_death_shoot_game_mode self) ; 请求Spawn
    )))

(event Custom|UpdateValues
  (params (Values :type Array%20of%20Death%20Shoot%20Player%20Data%20Structures))
  ;[1 0.9161 0.2633] 拿到数据 放入排行榜UI里  刷新排行榜UI
  (bind _output_get (Variables|Default|SetValues Values))
  (Class|KismaetMultiFPSLibrary|SortValues _output_get) ; C++实现排序
  (bind _playeui (Variables|Default|GetPlayeUI) ; 拿到PlayerUI
    (:then
      (Default|UpdateSortBox _playeui (Variables|Default|GetValues)) ; 调用UI刷新的这个方法
    )
    (:else)))

(event Custom|ServerRequireUpdate
  ;[1 0.9161 0.2633] 拿到服务器的GameMode 调用UpdateValues
  (bind _asbp_death_shoot_game_mode (Utilities|Casting|CastToBP_DeathShootGameMode (Game|GetGameMode)))
  (Default|UpdateValues _asbp_death_shoot_game_mode))

(event Custom|ClientUpdateDownTime
  (params (DownTime :type Integer))
  ;[1 1 1] 开始计时
  (Variables|Default|SetDownTime DownTime))

(event Custom|ClientDisableInput
  ;[1 0.4129 0.5271] 死亡时候禁止客户端上玩家输入
  (Input|DisableInput (Pawn|GetControlledPawn) self))

(event Custom|ClientEndGame
  ;[1 1 1] 所有客户端上执行 回到主菜单
  (Game|OpenLevel(byName) "MainMenu"))

(event Custom|ClientHidMouse
  ;[1 1 1] 游戏开始隐藏鼠标
  (Input|SetInputModeGameOnly self)
  (Variables|Default|SetbShowMouseCursor false))

(event EventDoCrosshairRecoil
  ;[1 1 1] UI
  ;;[0.9478 0.3532 1] 播放十字扩散动画
  (Default|DoCrosshairRecoil (Variables|Default|GetPlayeUI)))

(event EventUpdateAmmoUI
  (params (ClipCurrentAmmo :type Integer) (GunCurrentAmmo :type Integer))
  ;[1 1 1] UI
  ;;[0.9478 0.3532 1] 子弹UI
  (Default|UpdateAmmo (Variables|Default|GetPlayeUI) ClipCurrentAmmo GunCurrentAmmo))

(event EventCreatePlayerUI
  ;[1 1 1] UI
  ;;[0.9478 0.3532 1] 游戏一开始显示UI
  (Variables|Default|GetPlayeUI
    (:then
      (Widget|RemovefromParent (Variables|Default|GetPlayeUI))
      (if (Pawn|IsLocalPlayerController)
        (bind _returnvalue (UserInterface|CreateWidget "/Game/Blueprints/GameUI/PlayerUI/WBP_PlayerUI.WBP_PlayerUI_C" self))
        (bind _output_get (Variables|Default|SetPlayeUI _returnvalue)) ; 保存起来
        (UserInterface|Viewport|AddtoViewport _output_get 0)
        ;;[1 0.9161 0.2633] 掉用服务器上的这个方法
        (CallFunction|ServerRequireUpdate)))
    (:else
      (if (Pawn|IsLocalPlayerController)
        (bind _returnvalue_2 (UserInterface|CreateWidget "/Game/Blueprints/GameUI/PlayerUI/WBP_PlayerUI.WBP_PlayerUI_C" self))
        (bind _output_get_2 (Variables|Default|SetPlayeUI _returnvalue_2)) ; 保存起来
        (UserInterface|Viewport|AddtoViewport _output_get_2 0)
        (CallFunction|ServerRequireUpdate)))))

(event EventUpdateHeathUI
  (params (NewHealth :type Float%20%28single-precision%29))
  ;[1 1 1] UI
  ;;[0.9478 0.3532 1] 血量更新
  (Default|UpdateHealth (Variables|Default|GetPlayeUI) NewHealth))

(event EventDeath
  (params (DamageActor :type Actor%20Object%20Reference))
  ;[1 0.4129 0.5271] Death逻辑
  (bind _asbp_death_shoot_game_mode (Utilities|Casting|CastToBP_DeathShootGameMode (Game|GetGameMode)))
  (Default|SelfDeath _asbp_death_shoot_game_mode self)
  (CallFunction|ClientDisableInput)
  (bind _aspc_fpsplayer_controller (Utilities|Casting|CastToPC_FPSPlayerController (Game|GetInstigatorController DamageActor)))
  (Default|KillAnother _asbp_death_shoot_game_mode _aspc_fpsplayer_controller)
  ;[1 0.4129 0.5271] 死亡后延迟0.2秒删除自己
  (Utilities|FlowControl|Delay 0.2)
  (Actor|DestroyActor (Pawn|GetControlledPawn))
  ;[1 0.4129 0.5271] 在重生
  (bind _asbp_death_shoot_game_mode_2 (Utilities|Casting|CastToBP_DeathShootGameMode (Game|GetGameMode)))
  (Utilities|IsValid _asbp_death_shoot_game_mode_2
    (:Is%20Valid
      (Default|RequstSpawn _asbp_death_shoot_game_mode_2 self) ; 请求Spawn
    )))

(fn ConstructionScript)