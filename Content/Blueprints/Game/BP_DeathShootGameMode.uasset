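; Game mode for a timed deathmatch shooter that handles player spawning, scoring and match end.
; The first PostLogin caches PlayerStarts and starts a one-second countdown pushed to every PC_FPSPlayerController, which calls ClientEndGame on them at zero.
; Each joining controller begins spawning and enters a score map, while RequstSpawn cycles through spawn points round-robin.
; Kills add points, deaths subtract them, and both rebroadcast the scoreboard to all players.
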(event Custom|RequstSpawn
  (params (PlayerController :type PC%20FPS%20Player%20Controller%20Object%20Reference))
  ;[1 1 1] SpawnActpr
  ;;[0.6337 0.6143 1] 生成玩家
  (Default|SpawnPlayerCharator PlayerController "/Game/Blueprints/Player/BP_PlayerPawn.BP_PlayerPawn_C" (Transformation|GetActorTransform (Utilities|Array|Get(acopy) (Variables|Playerbirthpointrelatedvariables|GetCharacterSpawnPoint) (Variables|Playerbirthpointrelatedvariables|GetSpawnIndex))))
  (Variables|Playerbirthpointrelatedvariables|SetSpawnIndex (+ (Variables|Playerbirthpointrelatedvariables|GetSpawnIndex) 1))
  (if (>= (Variables|Playerbirthpointrelatedvariables|GetSpawnIndex) (Utilities|Array|Length (Variables|Playerbirthpointrelatedvariables|GetCharacterSpawnPoint)))
    (Variables|Playerbirthpointrelatedvariables|SetSpawnIndex 0) ; 超过数组长度归零
  ))

(event Custom|UpdateValues
  ;[1 0.9161 0.2633] 刷新排行界面
  (bind _keys (Utilities|Map|Keys (Variables|PlayerGameDataMap|GetPlayerGameDataMap))) ; 拿到所有的PlayerController
  (for _array_element _keys
    (bind _values (Utilities|Map|Values (Variables|PlayerGameDataMap|GetPlayerGameDataMap)))
    (Default|UpdateValues _array_element _values)))

(event Custom|KillAnother
  (params (PlayerController :type PC%20FPS%20Player%20Controller%20Object%20Reference))
  (bind _playergamedatamap (Variables|PlayerGameDataMap|GetPlayerGameDataMap))
  (bind _value (Utilities|Map|Find _playergamedatamap PlayerController))
  (bind (_playername _playerscore) (Utilities|Struct|BreakDeathShootPlayerData _value))
  ;[1 1 1] 死亡后的逻辑
  ;;[1 0.4129 0.5271] 杀死别人
  (Variables|KillOtherUpdateValue|SetKillOtherShortName _playername)
  (Variables|KillOtherUpdateValue|SetKillOtherShortScore (+ _playerscore 15))
  (Utilities|Map|Remove (Variables|PlayerGameDataMap|GetPlayerGameDataMap) PlayerController)
  (Utilities|Map|Add (Variables|PlayerGameDataMap|GetPlayerGameDataMap) PlayerController (Utilities|Struct|MakeDeathShootPlayerData (Variables|KillOtherUpdateValue|GetKillOtherShortName) (Variables|KillOtherUpdateValue|GetKillOtherShortScore)))
  ;;[1 0.9161 0.2633] 刷新UI
  (CallFunction|UpdateValues))

(event Custom|SelfDeath
  (params (PlayerController :type PC%20FPS%20Player%20Controller%20Object%20Reference))
  (bind _playergamedatamap (Variables|PlayerGameDataMap|GetPlayerGameDataMap))
  (bind _value (Utilities|Map|Find _playergamedatamap PlayerController))
  (bind (_playername _playerscore) (Utilities|Struct|BreakDeathShootPlayerData _value))
  ;[1 1 1] 死亡后的逻辑
  ;;[1 0.4129 0.5271] 自己死的时候把自己的数据找出来 短暂的存一下  然后把自己删了 在加回去 值就改变了
  (Variables|SelfDeathUpdateValue|SetHirtPlayerShortName _playername)
  (Variables|SelfDeathUpdateValue|SetHirtPlayerShortScore (- _playerscore 10))
  (Utilities|Map|Remove (Variables|PlayerGameDataMap|GetPlayerGameDataMap) PlayerController)
  (Utilities|Map|Add (Variables|PlayerGameDataMap|GetPlayerGameDataMap) PlayerController (Utilities|Struct|MakeDeathShootPlayerData (Variables|SelfDeathUpdateValue|GetHirtPlayerShortName) (Variables|SelfDeathUpdateValue|GetHirtPlayerShortScore)))
  ;;[1 0.9161 0.2633] 刷新UI
  (CallFunction|UpdateValues))

(event Custom|GameStateSet
  ;[1 1 1] 游戏开始设定
  ;;[1 1 1] 第一个玩家加入时去Get所有的出生点
  (bind _outactors (Actor|GetAllActorsOfClass "/Script/Engine.PlayerStart"))
  (Variables|Playerbirthpointrelatedvariables|SetCharacterSpawnPoint _outactors)
  (bind _returnvalue (Utilities|Time|SetTimerbyEvent (delegate Custom|Down) 1.0 true))
  (Variables|Timer|SetDownTimerHandle _returnvalue))

(event Custom|Down
  ;[1 1 1] 游戏开始设定
  ;;[1 1 1] 倒计时开始
  (Variables|Timer|SetRoundTime (- (Variables|Timer|GetRoundTime) 1))
  ;;[1 1 1] 所有玩家客户端UI更新时间
  (bind _keys (Utilities|Map|Keys (Variables|PlayerGameDataMap|GetPlayerGameDataMap)))
  (for _array_element _keys
    (Default|ClientUpdateDownTime _array_element (Variables|Timer|GetRoundTime)) ; 所有玩家刷新DownTimeUI
  )
  ;;[1 1 1] 时间归0 游戏结束
  (if (<= (Variables|Timer|GetRoundTime) 0)
    (Utilities|Time|ClearandInvalidateTimerbyHandle (Variables|Timer|GetDownTimerHandle)) ; 游戏结束 清空
    (CallFunction|EndGame)))

(event Custom|EndGame
  ;[1 0 0] EndGame
  (bind _keys (Utilities|Map|Keys (Variables|PlayerGameDataMap|GetPlayerGameDataMap)))
  (for _array_element _keys
    (Default|ClientEndGame _array_element)))

(event EventPostLogin
  (params (NewPlayer :type Player%20Controller%20Object%20Reference))
  ;[1 1 1] SpawnActpr
  ;;[1 1 1] 第一个玩家加入就Set计时器 然后Spwan自己
  (if (Variables|Timer|GetFristCharcterJionGame)
    _
    (else
      (CallFunction|GameStateSet)
      (Variables|Timer|SetFristCharcterJionGame true)))
  ;;[0.6337 0.6143 1] 玩家加载进入时候 生成一个Character 作为PlayerController控制的Pawn
  (bind _aspc_fpsplayer_controller (Utilities|Casting|CastToPC_FPSPlayerController NewPlayer)) ; 转换为我们自己的PlayerController类型
  (Utilities|IsValid _aspc_fpsplayer_controller ; 判断是否成功
    (:Is%20Valid
      (Default|StartSpawnCharator _aspc_fpsplayer_controller)
      ;;[1 0.9161 0.2633] 记录进来玩家的名字分数
      (Utilities|Map|Add (Variables|PlayerGameDataMap|GetPlayerGameDataMap) _aspc_fpsplayer_controller (Utilities|Struct|MakeDeathShootPlayerData (Utilities|String|StringToName (Utilities|GetObjectName _aspc_fpsplayer_controller)))))))

(fn ConstructionScript)