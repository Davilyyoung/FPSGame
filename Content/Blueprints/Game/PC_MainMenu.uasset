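; Main menu player controller that shows the title screen at game start and switches to the main menu, noted in a comment as the search interface.
; BeginPlay creates the title widget, adds it to the viewport and shows the mouse cursor.
; Pressing Space removes the title, creates and displays the main menu widget, then sets UI-only input with the mouse always locked.
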(event EventBeginPlay
  ;[1 1 1] 游戏一开始界面
  (bind _returnvalue (UserInterface|CreateWidget "/Game/Blueprints/GameUI/MainUI/WBP_TitleUI.WBP_TitleUI_C" self))
  (bind _output_get (Variables|Default|SetMain _returnvalue))
  (UserInterface|Viewport|AddtoViewport _output_get 0)
  (Variables|Default|SetbShowMouseCursor true))

(event Input|KeyboardEvents|SpaceBar
  (params (Key :type Key%20Structure :default "None"))
  ;[1 1 1] 搜索界面
  (:Pressed
    (Widget|RemovefromParent (Variables|Default|GetMain))
    (bind _returnvalue (UserInterface|CreateWidget "/Game/Blueprints/GameUI/MainUI/WBP_MainMenuUI.WBP_MainMenuUI_C" self))
    (bind _output_get (Variables|Default|SetMainMenu _returnvalue))
    (UserInterface|Viewport|AddtoViewport _output_get 0)
    (Input|SetInputModeUIOnly self 0 "LockAlways")
    (Variables|Default|SetbShowMouseCursor true)))

(fn ConstructionScript)