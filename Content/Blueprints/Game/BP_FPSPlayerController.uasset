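; BP_FPSPlayerController is the FPS player controller that owns the player's HUD widget.
; CreatePlayerUI builds WBP_PlayerUI only for a local controller, stores it and adds it to the viewport.
; Its other custom events forward crosshair recoil, clip and gun ammo counts, and health changes to that widget.
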(event EventDoCrosshairRecoil
  ;[1 1 1] 播放十字扩散动画
  (Default|DoCrosshairRecoil (Variables|Default|GetPlayeUIr)))

(event EventUpdateAmmoUI
  (params (ClipCurrentAmmo :type Integer) (GunCurrentAmmo :type Integer))
  ;[1 1 1] 子弹UI
  (Default|UpdateAmmo (Variables|Default|GetPlayeUIr) ClipCurrentAmmo GunCurrentAmmo))

(event EventCreatePlayerUI
  ;[1 1 1] 游戏一开始显示UI
  (if (Pawn|IsLocalPlayerController)
    (bind _returnvalue (UserInterface|CreateWidget "/Game/Blueprints/GameUI/WBP_PlayerUI.WBP_PlayerUI_C" self))
    (bind _output_get (Variables|Default|SetPlayeUIr _returnvalue)) ; 保存起来
    (UserInterface|Viewport|AddtoViewport _output_get 0)))

(event EventUpdateHeathUI
  (params (NewHealth :type Float%20%28single-precision%29))
  ;[1 1 1] 血量更新
  (Default|UpdateHealth (Variables|Default|GetPlayeUIr) NewHealth))

(fn ConstructionScript)